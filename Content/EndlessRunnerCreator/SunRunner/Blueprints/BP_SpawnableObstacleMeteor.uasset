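; Meteor obstacle for the SunRunner endless runner, extending a parent spawnable with randomised visuals.
; EnableObject randomises mesh, scale and yaw, then calls the parent implementation.
; A rare roll boosts the dynamic material's emissive strength, though both mesh options are currently the same CometMesh.
; Scale is random per axis within MinSize and MaxSize, applied to the mesh rather than the actor so it grows from its pivot.
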(event `self.ReceiveBeginPlay`
  (`parent.ReceiveBeginPlay`))

(fn `EnableObject`
  ;[0 0 0] Randomise the object mesh, scale and rotations.
  (`self.SetRandomStaticMesh`)
  (`self.SetRandomActorScale`)
  (`self.SetRandomActorRotation`)
  (`parent.EnableObject`))

(fn `SetRandomActorRotation`
  (`self.K2_SetActorRotation` (`KismetMathLibrary.MakeRotator` 0.0 0.0 (`KismetMathLibrary.RandomFloatInRange` 0.0 360.0))))

(fn `SetRandomActorScale`
  ;[0 0 0] Apply random scale to the static mesh. Apply it to the Mesh not the Object so we can make use of scaling from the pivot point to scale up and out from bottom/middle rather than middle/middle.
  (`SceneComponent.SetWorldScale3D` (`self.StaticMesh`) (`KismetMathLibrary.MakeVector` (`KismetMathLibrary.RandomFloatInRange` (`self.MinSize`) (`self.MaxSize`)) (`KismetMathLibrary.RandomFloatInRange` (`self.MinSize`) (`self.MaxSize`)) (`KismetMathLibrary.RandomFloatInRange` (`self.MinSize`) (`self.MaxSize`)))))

(fn `SetRandomStaticMesh`
  (locals (bUseSpecialObstacleMesh :type Boolean :default false))
  (set `local.bUseSpecialObstacleMesh` (> (`KismetMathLibrary.RandomIntegerInRange` 0 10) 9))
  ;[0 0 0] Set the static mesh to a random mesh.
  (`StaticMeshComponent.SetStaticMesh` (`self.StaticMesh`) (select `int` (select `bool` (`local.bUseSpecialObstacleMesh`) :`true` 1) :`0` "/Game/EndlessRunnerCreator/SunRunner/CometModel/CometBreak/CometMesh.CometMesh" :`1` "/Game/EndlessRunnerCreator/SunRunner/CometModel/CometBreak/CometMesh.CometMesh" :!type "StaticMesh Object Reference"))
  ;[0 0 0] If using "Special Mesh" Increase the Emissive Strenght just for visual purposes.
  ; Otherwise use the standard EmissiveStrength
  (`MaterialInstanceDynamic.SetScalarParameterValue` (`self.DynamicMaterialInstance`) "EmissiveStrength" (select `bool` (`local.bUseSpecialObstacleMesh`) :`false` 1.0 :`true` 10.0 :!type "Float (single-precision)")))

(fn `UserConstructionScript`
  (`parent.UserConstructionScript`))