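; Spawnable cone obstacle for SunRunner that penalizes the player on contact.
; On enable it gets a random yaw, a fixed mesh scale and an occasional brighter emissive "special" variant, though both variants use the same cone mesh.
; HitPlayer sets explosion effects, shrinks the player, cuts score and combo, then calls the parent.
; MovetoPlayer is overridden empty so magnet pickups do not attract it.
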(event `self.ReceiveBeginPlay`
  (`parent.ReceiveBeginPlay`))

(event `self.MoveToPlayer`
  ;[0 0 0 1 40] Override the command in parent and tell it to do nothing when magnet is picked up
)

(fn `CallAddCurrency`
  (params (CurrencyToAdd :type Integer))
  (returns (Return :type Boolean))
  (return false))

(fn `CallAddLife`
  (params (LivesToAdd :type Integer))
  (returns (Return :type Boolean))
  (return false))

(fn `CallGetCurrentGameState`
  (returns (CurrentGameState :type "/Game/EndlessRunnerCreator/CommonAssets/Blueprints/Enums/EGameState Enum"))
  (return "NewEnumerator0"))

(fn `CallGetScore`
  (returns (CurrentScore :type Integer))
  (return 0))

(fn `CallPausePressed`
  (returns (Return :type Boolean))
  (return false))

(fn `CallPlayerDied`
  (params (PlayerRef :type "Actor Object Reference"))
  (returns (Return :type Boolean))
  (return false))

(fn `CallSetGameState`
  (params (CurrentState :type "/Game/EndlessRunnerCreator/CommonAssets/Blueprints/Enums/EGameState Enum" :default "NewEnumerator0"))
  (returns (Return :type Boolean))
  (return false))

(fn `CallSetLevelHUDRef`
  (params (LevelHUD :type "/Game/EndlessRunnerCreator/CommonAssets/Blueprints/UI/WBP_HUDBase Object Reference"))
  (returns (Return :type Boolean))
  (return false))

(fn `CallSetLevelManager`
  (params (LevelManager :type "/Game/EndlessRunnerCreator/CommonAssets/Blueprints/Game/BP_LevelManagerBase Object Reference"))
  (returns (Return :type Boolean))
  (return false))

(fn `CallSetMaxLives`
  (params (Lives :type Integer))
  (returns (Return :type Boolean))
  (return false))

(fn `CallSetRespawnDelay`
  (params (RespawnDelay :type "Float (double-precision)"))
  (returns (Return :type Boolean))
  (return false))

(fn `CallSetScore`
  (params (Score :type Integer))
  (returns (Return :type Boolean))
  (return false))

(fn `EnableObject`
  ;[0 0 0] Randomise the object mesh, scale and rotations.
  (`self.SetRandomStaticMesh`)
  (`self.SetRandomActorScale`)
  (`self.SetRandomActorRotation`)
  (`parent.EnableObject`))

(fn `HitPlayer`
  (set `self.HitSound` "/Game/EndlessRunnerCreator/CommonAssets/Audio/Impact_Cue_Audio.Impact_Cue_Audio")
  (set `self.HitNiagaraSystem` "/Game/EndlessRunnerCreator/SunRunner/Effects/Particle_Systems/VFX_Cone_Explosion.VFX_Cone_Explosion")
  (bind _asbp_player_sun_runner (cast `/Game/EndlessRunnerCreator/SunRunner/Blueprints/BP_PlayerSunRunner` (`GameplayStatics.GetPlayerPawn` 0))
    (:`then`
      (bind (_player_scale_x _player_scale_y _player_scale_z) (`KismetMathLibrary.BreakVector` (`/Game/EndlessRunnerCreator/SunRunner/Blueprints/BP_PlayerSunRunner.Player Scale` _asbp_player_sun_runner)))
      (`/Game/EndlessRunnerCreator/SunRunner/Blueprints/BP_PlayerSunRunner.ResizeSmaller` _asbp_player_sun_runner (/ _player_scale_z 3.0))
      (`/Game/EndlessRunnerCreator/CommonAssets/Blueprints/Game/BP_LevelManagerBase.SubtractToScore` (`self.LevelManagerRef`) 300.0)
      ;[1 1 1] Combo Code
      (`/Game/EndlessRunnerCreator/SunRunner/Blueprints/BP_PlayerSunRunner.DecreaseComboMeter` _asbp_player_sun_runner)
      (`parent.HitPlayer`))
    (:`CastFailed`
      (`KismetSystemLibrary.PrintString` "Hello"))))

(fn `SetRandomActorRotation`
  (`self.K2_SetActorRotation` (`KismetMathLibrary.MakeRotator` 0.0 0.0 (`KismetMathLibrary.RandomFloatInRange` 0.0 360.0))))

(fn `SetRandomActorScale`
  ;[0 0 0] Apply random scale to the static mesh. Apply it to the Mesh not the Object so we can make use of scaling from the pivot point to scale up and out from bottom/middle rather than middle/middle.
  (`SceneComponent.SetWorldScale3D` (`self.StaticMesh`) (1.5 1.5 1.5)))

(fn `SetRandomStaticMesh`
  (locals (bUseSpecialObstacleMesh :type Boolean :default false))
  (set `local.bUseSpecialObstacleMesh` (> (`KismetMathLibrary.RandomIntegerInRange` 0 10) 9))
  ;[0 0 0] Set the static mesh to a random mesh.
  (`StaticMeshComponent.SetStaticMesh` (`self.StaticMesh`) (select `int` (select `bool` (`local.bUseSpecialObstacleMesh`) :`true` 1) :`0` "/Game/EndlessRunnerCreator/SunRunner/MobileStarterContent/Shapes/Shape_Cone.Shape_Cone" :`1` "/Game/EndlessRunnerCreator/SunRunner/MobileStarterContent/Shapes/Shape_Cone.Shape_Cone" :!type "StaticMesh Object Reference"))
  ;[0 0 0] If using "Special Mesh" Increase the Emissive Strenght just for visual purposes.
  ; Otherwise use the standard EmissiveStrength
  (`MaterialInstanceDynamic.SetScalarParameterValue` (`self.DynamicMaterialInstance`) "EmissiveStrength" (select `bool` (`local.bUseSpecialObstacleMesh`) :`false` 7.0 :`true` 10.0 :!type "Float (single-precision)")))

(fn `UserConstructionScript`
  (`parent.UserConstructionScript`))