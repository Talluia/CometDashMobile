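; Meteor pickup for the endless runner that grows the sun player when collected, built on a parent spawnable pickup.
; EnableObject applies the comet mesh, a random rotation and clamped random scales around the player's MaxScale, rolling MeteorScale separately.
; HitPlayer sets break VFX, raises combo, size and score, and sends an add-life message before calling the parent.
; The meteor-versus-player size comparison and size-bar UI update are disconnected.
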(fn `CallAddCurrency`
  (params (CurrencyToAdd :type Integer))
  (returns (Return :type Boolean))
  (return false))

(fn `CallAddLife`
  (params (LivesToAdd :type Integer))
  (returns (Return :type Boolean))
  (return false))

(fn `CallGetCurrentGameState`
  (returns (CurrentGameState :type "/Game/EndlessRunnerCreator/CommonAssets/Blueprints/Enums/EGameState Enum"))
  (return "NewEnumerator0"))

(fn `CallGetScore`
  (returns (CurrentScore :type Integer))
  (return 0))

(fn `CallPausePressed`
  (returns (Return :type Boolean))
  (return false))

(fn `CallPlayerDied`
  (params (PlayerRef :type "Actor Object Reference"))
  (returns (Return :type Boolean))
  (return false))

(fn `CallSetGameState`
  (params (CurrentState :type "/Game/EndlessRunnerCreator/CommonAssets/Blueprints/Enums/EGameState Enum" :default "NewEnumerator0"))
  (returns (Return :type Boolean))
  (return false))

(fn `CallSetLevelHUDRef`
  (params (LevelHUD :type "/Game/EndlessRunnerCreator/CommonAssets/Blueprints/UI/WBP_HUDBase Object Reference"))
  (returns (Return :type Boolean))
  (return false))

(fn `CallSetLevelManager`
  (params (LevelManager :type "/Game/EndlessRunnerCreator/CommonAssets/Blueprints/Game/BP_LevelManagerBase Object Reference"))
  (returns (Return :type Boolean))
  (return false))

(fn `CallSetMaxLives`
  (params (Lives :type Integer))
  (returns (Return :type Boolean))
  (return false))

(fn `CallSetRespawnDelay`
  (params (RespawnDelay :type "Float (double-precision)"))
  (returns (Return :type Boolean))
  (return false))

(fn `CallSetScore`
  (params (Score :type Integer))
  (returns (Return :type Boolean))
  (return false))

(fn `EnableObject`
  (bind _returnvalue (`KismetMathLibrary.RandomFloatInRange` 0.0 360.0))
  (bind _returnvalue_2 (`KismetMathLibrary.FClamp` (`KismetMathLibrary.RandomFloatInRange` (`self.MeteorMin`) (`self.MeteorMax`)) 1.0 7.0))
  (bind (_max_scale_x _max_scale_y _max_scale_z) (`KismetMathLibrary.BreakVector` (`/Game/EndlessRunnerCreator/SunRunner/Blueprints/BP_PlayerSunRunner.Max Scale` (cast `/Game/EndlessRunnerCreator/SunRunner/Blueprints/BP_PlayerSunRunner` (`GameplayStatics.GetPlayerPawn` 0) :!pure true))))
  (bind _returnvalue_3 (`KismetMathLibrary.MakeVector` _returnvalue_2 _returnvalue_2 _returnvalue_2))
  (set `self.MeteorMin` (- _max_scale_z 0.2))
  (set `self.MeteorMax` (+ _max_scale_z 0.2))
  (`StaticMeshComponent.SetStaticMesh` (`self.StaticMesh`) "/Game/EndlessRunnerCreator/SunRunner/CometModel/CometBreak/CometMesh.CometMesh")
  (`SceneComponent.SetWorldScale3D` (`self.Scene`) _returnvalue_3)
  (set `self.MeteorScale` _returnvalue_3)
  (`self.K2_SetActorRotation` (`KismetMathLibrary.MakeRotator` _returnvalue _returnvalue _returnvalue))
  (`parent.EnableObject`))

(fn `HitPlayer`
  (set `self.HitNiagaraSystem` "/Game/EndlessRunnerCreator/SunRunner/Effects/Particle_Systems/VFX_Obstacle_Break.VFX_Obstacle_Break")
  (bind _asbp_player_sun_runner (cast `/Game/EndlessRunnerCreator/SunRunner/Blueprints/BP_PlayerSunRunner` (`GameplayStatics.GetPlayerPawn` 0)))
  ;[1 1 1] COMBO CODE
  (`/Game/EndlessRunnerCreator/SunRunner/Blueprints/BP_PlayerSunRunner.IncreaseComboMeter` _asbp_player_sun_runner 1)
  (`/Game/EndlessRunnerCreator/SunRunner/Blueprints/BP_PlayerSunRunner.ResizeBigger` _asbp_player_sun_runner 2.0)
  (`/Game/EndlessRunnerCreator/CommonAssets/Blueprints/Game/BP_LevelManagerBase.AddToScore` (`self.LevelManagerRef`))
  (message `/Game/EndlessRunnerCreator/CommonAssets/Blueprints/Interfaces/BPI_GameMode.CallAddLife` (`GameplayStatics.GetGameMode`) (`self.LivesValue`))
  (`/Game/EndlessRunnerCreator/SunRunner/Blueprints/BP_PlayerSunRunner.IncreasePlayerScale` _asbp_player_sun_runner)
  (`parent.HitPlayer`))

(fn `UserConstructionScript`
  (`parent.UserConstructionScript`))