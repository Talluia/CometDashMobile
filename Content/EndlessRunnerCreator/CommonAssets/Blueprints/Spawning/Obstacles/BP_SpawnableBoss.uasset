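; Spawnable boss ship for the Sun Runner endless runner that pits its size against the player's.
; On enable it takes a random scale from bounds based on player max scale and sets up its size widget.
; Tick tints that bar red or green, fires a homing missile and resets speed offset after delays.
; On hit, the player's size check either shrinks the player or grows them and clears obstacles and missiles.
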(event `ChangeTextColor`
  (bind (_bossscale_x _bossscale_y _bossscale_z) (`KismetMathLibrary.BreakVector` (`self.BossScale`)))
  ;[0 0.7546 1 1 40] Boss Mechanics
  ;;[0 0.7834 1 1 30] Change Material Color
  (bind _asbp_player_sun_runner (cast `/Game/EndlessRunnerCreator/SunRunner/Blueprints/BP_PlayerSunRunner` (`GameplayStatics.GetPlayerPawn` 0)))
  (bind _asui_ship_size_needed (cast `/Game/EndlessRunnerCreator/CommonAssets/Blueprints/UI/UI_Ship_Size_Needed` (`WidgetComponent.GetWidget` (`self.SizeNeeded`))))
  (bind _size_progressbar (`/Game/EndlessRunnerCreator/CommonAssets/Blueprints/UI/UI_Ship_Size_Needed.Size_ProgressBar` _asui_ship_size_needed))
  (bind (_backgroundimage _fillimage _marqueeimage) (break `ProgressBarStyle` (`ProgressBar.WidgetStyle` _size_progressbar)))
  (bind (_imagesize _margin _tintcolor _resourceobject) (break `SlateBrush` _fillimage))
  (bind (_player_scale_x _player_scale_y _player_scale_z) (`KismetMathLibrary.BreakVector` (`/Game/EndlessRunnerCreator/SunRunner/Blueprints/BP_PlayerSunRunner.Player Scale` _asbp_player_sun_runner)))
  (set `ProgressBar.WidgetStyle` (make `ProgressBarStyle` _backgroundimage (make `SlateBrush` _imagesize _margin (select `bool` (>= _bossscale_z _player_scale_z) :`false` (make `SlateColor` (struct :`G` 1.0 :`B` 0.084725 :`A` 1.0)) :`true` (make `SlateColor` (struct :`R` 1.0 :`B` 0.016751 :`A` 1.0))) _resourceobject) _marqueeimage) _size_progressbar))

(event `self.ReceiveTick`
  (params (DeltaSeconds :type "Float (single-precision)"))
  (bind (_returnvalue_location _returnvalue_rotation) (`KismetMathLibrary.BreakTransform` (`SceneComponent.K2_GetComponentToWorld` (`self.RocketSpawner`))))
  ;[1 0.2099 0 1 40] EVENT TICK
  (`parent.ReceiveTick` DeltaSeconds)
  (`self.ChangeTextColor`)
  (`|ExecutionSequence`
    (:`then_0`
      ;;[1 1 1] Make it boolean
      (`KismetSystemLibrary.Delay` 10.0)
      ;;[1 1 1] Set the Boss speed to Level speed to make the boss move forward
      (set `self.SpeedOffset` 0.0))
    (:`then_1`
      (`KismetSystemLibrary.Delay` 2.0)
      (if (> (`self.Rocket Ammo`) 0)
        (set `self.Rocket Ammo` (- (`self.Rocket Ammo`) 1))
        (bind _returnvalue (`|SpawnActorFromClass` "/Game/EndlessRunnerCreator/SunRunner/HomingProjectile/EndlessHomingMissile.EndlessHomingMissile_C" (`KismetMathLibrary.MakeTransform` _returnvalue_location _returnvalue_rotation) "Undefined" "OverrideRootScale" null true null))
        (bind _asbp_player_sun_runner (cast `/Game/EndlessRunnerCreator/SunRunner/Blueprints/BP_PlayerSunRunner` (`GameplayStatics.GetPlayerPawn` 0)))
        (set `/Game/EndlessRunnerCreator/SunRunner/HomingProjectile/EndlessHomingMissile.Target` _asbp_player_sun_runner _returnvalue)))
    (:`then_2`
      (bind _asbp_player_sun_runner_2 (cast `/Game/EndlessRunnerCreator/SunRunner/Blueprints/BP_PlayerSunRunner` (`GameplayStatics.GetPlayerPawn` 0)))
      (set `self.BossHealthPercentage` (`/Game/EndlessRunnerCreator/SunRunner/Blueprints/BP_PlayerSunRunner.UI_LifePercentageDivider` _asbp_player_sun_runner_2)))
    (:`then_3`
      (`self.UpdateBossScale`))))

(event `self.ReceiveBeginPlay`
  ;[0 0.09229 1 1 40] Event Begin Play
  (`parent.ReceiveBeginPlay`)
  (set `self.HitSound` "/Game/EndlessRunnerCreator/CommonAssets/Audio/Ambience/CD_Ambience_PlanetExplosion_02.CD_Ambience_PlanetExplosion_02")
  (bind _asbp_player_sun_runner (cast `/Game/EndlessRunnerCreator/SunRunner/Blueprints/BP_PlayerSunRunner` (`GameplayStatics.GetPlayerPawn` 0)))
  (set `self.PlayerRef` _asbp_player_sun_runner))

(event `UpdateBossScale`
  ;[0 0.7546 1 1 40] Boss Mechanics
  ;;[1 1 1] Update Boss Scale  |  Cast to Player  |  Sets BossMaxScale to Player MaxScale  |  IF BossMaxScale = 1 Then BossMinScale is set to Player MinScale  |  IF BossMaxScale != 1 Then BossMinScale is set to Player MaxScale - 1
  (bind _asbp_player_sun_runner (cast `/Game/EndlessRunnerCreator/SunRunner/Blueprints/BP_PlayerSunRunner` (`GameplayStatics.GetPlayerPawn` 0)))
  (if (== (`self.BossMaxScale`) 1.0)
    (bind (_min_scale_x _min_scale_y _min_scale_z) (`KismetMathLibrary.BreakVector` (`/Game/EndlessRunnerCreator/SunRunner/Blueprints/BP_PlayerSunRunner.Min Scale` _asbp_player_sun_runner)))
    (set `self.BossMinScale` _min_scale_z)
    (bind (_max_scale_x _max_scale_y _max_scale_z) (`KismetMathLibrary.BreakVector` (`/Game/EndlessRunnerCreator/SunRunner/Blueprints/BP_PlayerSunRunner.Max Scale` _asbp_player_sun_runner)))
    (set `self.BossMaxScale` _max_scale_z)
    (else
      (set `self.BossMaxScale` (- _max_scale_z 0.7))
      (set `self.BossMinScale` (- _max_scale_z 1.0)))))

(event `self.StaticMesh.OnComponentHit`
  (params (HitComponent :type "PrimitiveComponent Object Reference") (OtherActor :type "Actor Object Reference") (OtherComp :type "PrimitiveComponent Object Reference") (NormalImpulse :type "Vector Structure") (Hit :type "HitResult Structure (by ref)"))
  ;[1 0.2708 0.8247 1 40] On Hit (StaticMesh)
  ;;[1 1 1] Hit Player
  (cast `/Game/EndlessRunnerCreator/SunRunner/Blueprints/BP_PlayerSunRunner` OtherActor)
  (`self.HitPlayer`))

(event `DestroyCones`
  ;[1 0.2708 0.8247 1 40] On Hit (StaticMesh)
  ;;[1 1 1] Destroy Cones  |  Gets all Cones in the Scene  |  Loops through & Calls Disable Object
  (`|ExecutionSequence`
    (:`then_0`
      (bind _outactors (`GameplayStatics.GetAllActorsOfClass` "/Game/EndlessRunnerCreator/SunRunner/Blueprints/BP_SpawnableObstacleSunRunner.BP_SpawnableObstacleSunRunner_C"))
      (for _array_element _outactors
        (`self.DisableObject` _array_element)
        (`GameplayStatics.PlayWorldCameraShake` "/Game/EndlessRunnerCreator/CommonAssets/Blueprints/CameraShake/BP_CameraShakeClearBoom.BP_CameraShakeClearBoom_C" (`self.K2_GetActorLocation`) 10000.0 100.0)
        (bind _returnvalue (`self.K2_GetActorLocation` _array_element))
        (`NiagaraFunctionLibrary.SpawnSystemAtLocation` "/Game/EndlessRunnerCreator/SunRunner/Effects/Particle_Systems/VFX_Cone_Explosion.VFX_Cone_Explosion" _returnvalue)
        (`GameplayStatics.PlaySoundAtLocation` "/Game/EndlessRunnerCreator/CommonAssets/Audio/CD_SFX_PowerUp_Shield_On_01.CD_SFX_PowerUp_Shield_On_01" _returnvalue (struct) 1.0 1.0 0.0 null null null))
      (`KismetArrayLibrary.Array_Clear` _outactors))
    (:`then_1`
      (bind _outactors_2 (`GameplayStatics.GetAllActorsOfClass` "/Game/EndlessRunnerCreator/SunRunner/HomingProjectile/EndlessHomingMissile.EndlessHomingMissile_C"))
      (for _array_element_2 _outactors_2
        (`self.DisableObject` _array_element_2))
      (`KismetArrayLibrary.Array_Clear` _outactors_2))))

(event `SetStaticMeshSize`
  (bind _staticmesh (`self.StaticMesh`))
  (bind (_clampx _clampy _clampz) (`self.ClampMaxScaleAxis` (`KismetMathLibrary.RandomFloatInRange` (`self.BossMinScale`) (`self.BossMaxScale`))))
  (bind _returnvalue (`KismetMathLibrary.MakeVector` _clampx _clampy _clampz))
  (`StaticMeshComponent.SetStaticMesh` _staticmesh "/Game/EndlessRunnerCreator/SunRunner/Meshes/Ship/MSH_BaddieSpaceShip_v2.MSH_BaddieSpaceShip_v2")
  (`SceneComponent.SetWorldScale3D` _staticmesh _returnvalue)
  (set `self.BossScale` _returnvalue)
  (`KismetSystemLibrary.PrintString` (`KismetStringLibrary.Conv_VectorToString` _returnvalue)))

(fn `CallGetMoveState`
  (returns (CurrentMoveState :type "/Game/EndlessRunnerCreator/CommonAssets/Blueprints/Enums/EMoveState Enum"))
  (return "NewEnumerator0"))

(fn `CallInvincibilityCollected`
  (params (InvincibilityDuration :type "Float (double-precision)" :default 0.0))
  (returns (Return :type Boolean))
  (return false))

(fn `CallIsObstacle`
  (returns (IsObstacle :type Boolean) (OverrideInvincibility :type Boolean))
  (return false false))

(fn `CallLevelStarted`
  (returns (Return :type Boolean))
  (return false))

(fn `CallMagnetCollected`
  (params (MagneticDuration :type "Float (double-precision)" :default 0.0))
  (returns (Return :type Boolean))
  (return false))

(fn `CallSetEnabled`
  (params (bEnabled :type Boolean))
  (returns (Return :type Boolean))
  (return false))

(fn `CallWasPlayerHit`
  (params (HitComponent :type "ActorComponent Object Reference"))
  (returns (PlayerHit :type Boolean))
  (return false))

(fn `EnableObject`
  (`self.UpdateBossScale`)
  (`self.SetStaticMeshSize`)
  (set `self.Rocket Ammo` 1)
  (set `self.SpeedOffset` -1000.0)
  ;[1 1 1] UI Set-up on Construction of the Enemy
  (bind _asbp_player_sun_runner (cast `/Game/EndlessRunnerCreator/SunRunner/Blueprints/BP_PlayerSunRunner` (`GameplayStatics.GetPlayerPawn` 0))
    (:`then`
      (bind _asui_ship_size_needed (cast `/Game/EndlessRunnerCreator/CommonAssets/Blueprints/UI/UI_Ship_Size_Needed` (`WidgetComponent.GetWidget` (`self.SizeNeeded`)))
        (:`then`
          (`ProgressBar.SetPercent` (`/Game/EndlessRunnerCreator/CommonAssets/Blueprints/UI/UI_Ship_Size_Needed.Size_ProgressBar` _asui_ship_size_needed) (`/Game/EndlessRunnerCreator/CommonAssets/Blueprints/UI/UI_Ship_Size_Needed.EnemyGetLifeSizePercent` _asui_ship_size_needed))
          (`/Game/EndlessRunnerCreator/CommonAssets/Blueprints/UI/UI_Ship_Size_Needed.Enemy_ResizeCallBack` _asui_ship_size_needed (`/Game/EndlessRunnerCreator/SunRunner/Blueprints/BP_PlayerSunRunner.SelectForSizeBar` _asbp_player_sun_runner) false)
          (set `/Game/EndlessRunnerCreator/CommonAssets/Blueprints/UI/UI_Ship_Size_Needed.BossRef` self _asui_ship_size_needed)
          (`parent.EnableObject`))
        (:`CastFailed`
          (`KismetSystemLibrary.PrintString` "Hello"))))
    (:`CastFailed`
      (`KismetSystemLibrary.PrintString` "Hello"))))

(fn `HitPlayer`
  (bind (_bossscale_x _bossscale_y _bossscale_z) (`KismetMathLibrary.BreakVector` (`self.BossScale`)))
  (bind _bosshealthpercentage (`self.BossHealthPercentage`))
  ;[1 1 1] Behavour for when the player is hit  |  What do we want to happen to the pawn when hit?  |  Destroy the player/kill player/Game over  |  SpawnablePickUp -> HitPlayer Function handles pickup animation etc..
  (bind _asbp_player_sun_runner (cast `/Game/EndlessRunnerCreator/SunRunner/Blueprints/BP_PlayerSunRunner` (`GameplayStatics.GetPlayerPawn` 0)))
  (bind (_player_scale_x _player_scale_y _player_scale_z) (`KismetMathLibrary.BreakVector` (`/Game/EndlessRunnerCreator/SunRunner/Blueprints/BP_PlayerSunRunner.Player Scale` _asbp_player_sun_runner)))
  (if (> _bossscale_z _player_scale_z)
    (`/Engine/EditorBlueprintResources/StandardMacros.DoOnce` false
      (:`Completed`
        (bind (_player_scale_x_2 _player_scale_y_2 _player_scale_z_2) (`KismetMathLibrary.BreakVector` (`/Game/EndlessRunnerCreator/SunRunner/Blueprints/BP_PlayerSunRunner.Player Scale` _asbp_player_sun_runner)))
        (`/Game/EndlessRunnerCreator/SunRunner/Blueprints/BP_PlayerSunRunner.ResizeSmaller` _asbp_player_sun_runner (/ _player_scale_z_2 4.0))
        (`/Game/EndlessRunnerCreator/SunRunner/Blueprints/BP_PlayerSunRunner.UpdatePlayerMaxScale` _asbp_player_sun_runner (-1.0 -1.0 -1.0))
        (`/Game/EndlessRunnerCreator/SunRunner/Blueprints/BP_PlayerSunRunner.ZoomOutCam` _asbp_player_sun_runner -20.0 0.0)
        (set `self.HitSound` "/Game/EndlessRunnerCreator/CommonAssets/Audio/Pickup_Audio.Pickup_Audio")
        (bind _result (`/Engine/EditorBlueprintResources/StandardMacros.DecrementFloat` _bosshealthpercentage)
          (:`  `
            (set `self.BossHealthPercentage` _result)
            (`/Game/EndlessRunnerCreator/SunRunner/Blueprints/BP_PlayerSunRunner.UpdateUI` _asbp_player_sun_runner 1.0)
            (`/Game/EndlessRunnerCreator/SunRunner/Blueprints/BP_PlayerSunRunner.UpdateComboRequirement` _asbp_player_sun_runner 1)
            ;;[1 1 1] Combo Code
            (`/Game/EndlessRunnerCreator/SunRunner/Blueprints/BP_PlayerSunRunner.DecreaseComboMeter` _asbp_player_sun_runner)))))
    (else
      (`/Engine/EditorBlueprintResources/StandardMacros.DoOnce` false
        (:`Completed`
          ;;[1 1 1] Enemy Combo Value
          (`/Game/EndlessRunnerCreator/SunRunner/Blueprints/BP_PlayerSunRunner.IncreaseComboMeter` _asbp_player_sun_runner 5)
          (set `self.HitSound` "/Game/EndlessRunnerCreator/CommonAssets/Audio/Ambience/CD_Ambience_PlanetExplosion_02.CD_Ambience_PlanetExplosion_02")
          (set `self.HitNiagaraSystem` "/Game/EndlessRunnerCreator/SunRunner/Effects/Particle_Systems/VFX_Player_Death.VFX_Player_Death")
          (`/Game/EndlessRunnerCreator/SunRunner/Blueprints/BP_PlayerSunRunner.ResizeBigger` _asbp_player_sun_runner 1.0)
          (`/Game/EndlessRunnerCreator/SunRunner/Blueprints/BP_PlayerSunRunner.IncreasePlayerScale` _asbp_player_sun_runner)
          (`self.DestroyCones`)
          (bind _result_2 (`/Engine/EditorBlueprintResources/StandardMacros.IncrementFloat` _bosshealthpercentage)
            (:`  `
              (set `self.BossHealthPercentage` _result_2)))))))
  (`self.UpdateBossScale`)
  (`parent.HitPlayer`))

(fn `ResizeBoss`
  (params (DamageDealt :type "Float (double-precision)"))
  (bind _staticmesh (`self.StaticMesh`))
  (bind (_returnvalue_x _returnvalue_y _returnvalue_z) (`KismetMathLibrary.BreakVector` (- (`SceneComponent.K2_GetComponentScale` _staticmesh) DamageDealt)))
  (bind _returnvalue (`KismetMathLibrary.FClamp` _returnvalue_x 1.0 7.0))
  (bind _returnvalue_2 (`KismetMathLibrary.FClamp` _returnvalue_y 1.0 7.0))
  (bind _returnvalue_3 (`KismetMathLibrary.FClamp` _returnvalue_z 1.0 7.0))
  (`SceneComponent.SetWorldScale3D` _staticmesh (`KismetMathLibrary.MakeVector` _returnvalue _returnvalue_2 _returnvalue_3))
  (set `self.BossScale` (`KismetMathLibrary.MakeVector` _returnvalue _returnvalue_2 _returnvalue_3)))

(fn `SetSpeed`)

(fn `SetStaticMesh`
  (returns (`Boss Scale` :type "Vector Structure")))

(fn `UserConstructionScript`
  (`parent.UserConstructionScript`))